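; BP_Boombox is an interactable boombox that the third-person character can switch on and off while standing next to it.
; It adds its own Enhanced Input mapping context, and box overlap events count nearby characters to gate the toggle input.
; A FlipFlop drives ToggleBoombox to pause or resume audio and swap the screen material.
; While on, a Timeline pulses the speakers' Y scale, restoring the saved default when off.
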(event OnComponentBeginOverlap(Box_Collision)
  (params (OverlappedComponent :type Primitive%20Component%20Object%20Reference) (OtherActor :type Actor%20Object%20Reference) (OtherComp :type Primitive%20Component%20Object%20Reference) (OtherBodyIndex :type Integer) (bFromSweep :type Boolean) (SweepResult :type Hit%20Result%20Structure%20%28by%20ref%29))
  ;[0.15 0.15 0.15 0.5] Get Overlapping Actors On Box Collision
  (CallFunction|SetOverlappingActors (Variables|Default|GetBox_Collision)))

(event OnComponentEndOverlap(Box_Collision)
  (params (OverlappedComponent :type Primitive%20Component%20Object%20Reference) (OtherActor :type Actor%20Object%20Reference) (OtherComp :type Primitive%20Component%20Object%20Reference) (OtherBodyIndex :type Integer))
  ;[0.15 0.15 0.15 0.5] Get Overlapping Actors Off Collision
  (CallFunction|SetOverlappingActors (Variables|Default|GetBox_Collision)))

(event Input|EnhancedActionEvents|EnhancedInputActionIA_Toggle_Boombox
  (params (ActionValue :type Boolean) (ElapsedSeconds :type Float%20%28double-precision%29) (TriggeredSeconds :type Float%20%28double-precision%29) (InputAction :type Input%20Action%20Object%20Reference :default "/Game/ELVTR/Inputs/IA_Toggle_Boombox.IA_Toggle_Boombox"))
  (bind _screen (Variables|Default|Getscreen))
  (bind _audio (Variables|Default|GetAudio))
  (bind _speakers (Variables|Default|Getspeakers))
  (:Started
    (Development|PrintString "Pressed f ")
    ;[0.15 0.15 0.15 0.5] Check if Overlapping
    (if (> (Variables|Default|GetOverlapped_Actors) 0)
      ;[0.15 0.15 0.15 0.5] Set Boombox On or Off
      (Utilities|FlowControl|FlipFlop
        (:A
          (bind _output_get (Variables|Default|SetOn_Off true))
          ;[0.15 0.15 0.15 0.5] Toggle Boombox
          (CallFunction|ToggleBoombox _output_get _audio _screen)
          (Development|PrintString "Boombox On")
          ;[0.15 0.15 0.15 0.5] Speaker Pulse Anim
          (bind _pulse_scale (Timeline|Timeline Play)
            (:Update
              (Transformation|SetRelativeScale3D _speakers (Math|Vector|MakeVector 1.0 _pulse_scale 1.0)))))
        (:B
          (bind _output_get_2 (Variables|Default|SetOn_Off false))
          (CallFunction|ToggleBoombox _output_get_2 _audio _screen)
          (Development|PrintString "Boombox Off")
          (Utilities|FlowControl|Sequence
            (:then_0
              (Timeline|Timeline Stop))
            (:then_1
              (Development|PrintString "resetting speakers")
              (Transformation|SetRelativeScale3D _speakers (Variables|Default|GetDefault_Speakers))))))
      (else
        (Development|PrintString "Not next to Boombox")))))

(event EventBeginPlay
  ;[0.15 0.15 0.15 0.5] Set Mapping Context
  (Input|AddMappingContext (PlayerController|LocalPlayerSubsystems|GetEnhancedInputLocalPlayerSubsystem (Game|GetPlayerController 0)) "/Game/ELVTR/Inputs/IMC_Boombox.IMC_Boombox" 0 "(bIgnoreAllPressedKeysUntilRelease=True,bForceImmediately=False,bNotifyUserSettings=False)")
  ;[0.15 0.15 0.15 0.5] Start Off
  (Rendering|Material|SetMaterial (Variables|Default|Getscreen) 0 "/Engine/MapTemplates/Materials/BasicAsset01.BasicAsset01")
  (Class|AudioComponent|SetPaused (Variables|Default|GetAudio) true)
  (Variables|Default|SetDefault_Speakers (Variables|/Script/Engine.SceneComponent|GetRelativeScale3D (Variables|Default|Getspeakers))))

(event Collision|EventActorBeginOverlap
  (params (OtherActor :type Actor%20Object%20Reference)))

(event EventTick
  (params (DeltaSeconds :type Float%20%28single-precision%29)))

(fn ConstructionScript)

(fn ToggleBoombox
  (params (On_Or_Off :type Boolean) (Sound :type Audio%20Component%20Object%20Reference) (Mesh :type Mesh%20Component%20Object%20Reference))
  ;[0.15 0.15 0.15 0.5] Toggle Sound
  (if On_Or_Off
    (Class|AudioComponent|SetPaused Sound false)
    ;[0.15 0.15 0.15 0.5] Toggle Screen
    (Rendering|Material|SetMaterial Mesh 0 "/Engine/MapTemplates/Materials/BasicAsset03.BasicAsset03")
    (else
      (Class|AudioComponent|SetPaused Sound true)
      (Rendering|Material|SetMaterial Mesh 0 "/Engine/MapTemplates/Materials/BasicAsset01.BasicAsset01"))))

(fn SetOverlappingActors
  (params (Collision :type Box%20Component%20Object%20Reference))
  ;[0.15 0.15 0.15 0.5] Set Overlapped Actors
  (bind _output_get (Variables|Default|SetOverlapped_Actors (Utilities|Array|Length (Collision|GetOverlappingActors Collision "/Game/ThirdPerson/Blueprints/BP_ThirdPersonCharacter.BP_ThirdPersonCharacter_C" :!class /Script/Engine.PrimitiveComponent))))
  ;[0.15 0.15 0.15 0.5] Print Overlapping Actors
  (Development|PrintString (Utilities|String|Append "Overlapping Actors:" (Utilities|String|ToString(Integer) _output_get))))