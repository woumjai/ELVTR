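; A three-point lighting rig actor that exposes key, fill and rim spotlight settings for editing on the placed instance.
; The construction script calls ModifyLight per light to set visibility, intensity, shadows, temperature, color and attenuation radius.
; Each light's target point is rotated by its pitch (negated) and yaw.
; All three lights share KeyAngle as outer cone angle, as ModifyLight ignores its Angle input.
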(event EventBeginPlay)

(event Collision|EventActorBeginOverlap
  (params (OtherActor :type Actor%20Object%20Reference)))

(event EventTick
  (params (DeltaSeconds :type Float%20%28single-precision%29)))

(fn ConstructionScript
  ;[0.15 0.15 0.15 0.5] Key Light
  (CallFunction|ModifyLight (Variables|Default|GetSpotLight_Key) (Variables|Key|GetKey%20On) (Variables|Key|GetKey%20Strength) (Variables|Key|GetKey%20Shadows) (Variables|Key|GetKey%20Temp) (Variables|Key|GetKey%20Color) (Variables|Default|GetTargetPoint_Key) (Variables|Key|GetKey%20%20Pitch) (Variables|Key|GetKey%20Yaw) (Variables|Key|GetKey%20Radius) 0.0)
  ;[0.15 0.15 0.15 0.5] Fill Light
  (CallFunction|ModifyLight (Variables|Default|GetSpotLight_Fill) (Variables|Fill|GetFill%20On) (Variables|Fill|GetFill%20Strength) (Variables|Fill|GetFill%20Shadows) (Variables|Fill|GetFill%20Temp) (Variables|Fill|GetFill%20Color) (Variables|Default|GetTargetPoint_Fill) (Variables|Fill|GetFill%20Pitch) (Variables|Fill|GetFill%20Yaw) (Variables|Fill|GetFill%20Radius) 0.0)
  ;[0.15 0.15 0.15 0.5] Rim Light
  (CallFunction|ModifyLight (Variables|rim|GetSpotLight_Rim) (Variables|Rim|GetRim%20On) (Variables|Rim|GetRim%20Strength) (Variables|Rim|GetRim%20Shadows) (Variables|Rim|GetRim%20Temp) (Variables|Rim|GetRim%20Color) (Variables|Default|GetTargetPoint_Rim) (Variables|Rim|GetRim%20Pitch) (Variables|Rim|GetRim%20Yaw) (Variables|Rim|GetRim%20Radius) 0.0))

(fn ModifyLight
  (params (Light :type Spot%20Light%20Component%20Object%20Reference) (On :type Boolean) (Strength :type Float%20%28double-precision%29) (Shadows :type Boolean) (Temperature :type Float%20%28double-precision%29) (Light%20Color :type Linear%20Color%20Structure) (Target%20Point :type Child%20Actor%20Component%20Object%20Reference) (Pitch :type Float%20%28double-precision%29) (Yaw :type Float%20%28double-precision%29) (Radius :type Float%20%28double-precision%29) (Angle :type Float%20%28double-precision%29))
  ;[0.15 0.15 0.15 0.5] Light Variables
  (Rendering|SetVisibility Light On false)
  (Rendering|Components|Light|SetIntensity Light Strength)
  (Rendering|Components|Light|SetCastShadows Light Shadows)
  (Class|LightComponent|SetTemperature Light Temperature)
  (Rendering|Components|Light|SetLightColor Light Light%20Color true)
  (Rendering|Lighting|SetAttenuationRadius Light Radius)
  (Rendering|Lighting|SetOuterConeAngle Light (Variables|Key|GetKey%20Angle))
  (Transformation|SetRelativeRotation Target%20Point (Math|Rotator|MakeRotator 0.0 (* Pitch -1.0) Yaw) false false))