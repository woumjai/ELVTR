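; Child Blueprint of a three-point light setup that can spin the whole rig around its vertical axis.
; On Tick, when DoRotation is set, it adds Speed as relative yaw to DefaultSceneRoot each frame, without scaling by delta time.
; The construction script and ModifyLight only forward to the parent, so light configuration is inherited unchanged.
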(event EventBeginPlay
  (|CallParentFunction) ; This node is disabled and will not be called.\nDrag off pins to build functionality.
)

(event Collision|EventActorBeginOverlap
  (params (OtherActor :type Actor%20Object%20Reference))
  (|CallParentFunction OtherActor) ; This node is disabled and will not be called.\nDrag off pins to build functionality.
)

(event EventTick
  (params (DeltaSeconds :type Float%20%28single-precision%29))
  (|CallParentFunction DeltaSeconds)
  (if (Variables|Rotation|GetDo%20Rotation)
    (Transformation|AddRelativeRotation (Variables|Default|GetDefaultSceneRoot) (Math|Rotator|MakeRotator 0.0 0.0 (Variables|Rotation|GetSpeed)) false false)))

(fn ConstructionScript
  (|CallParentFunction))

(fn ModifyLight
  (params (Light :type Spot%20Light%20Component%20Object%20Reference) (On :type Boolean) (Strength :type Float%20%28double-precision%29) (Shadows :type Boolean) (Temperature :type Float%20%28double-precision%29) (Light%20Color :type Linear%20Color%20Structure) (Target%20Point :type Child%20Actor%20Component%20Object%20Reference) (Pitch :type Float%20%28double-precision%29) (Yaw :type Float%20%28double-precision%29) (Radius :type Float%20%28double-precision%29) (Angle :type Float%20%28double-precision%29))
  (|CallParentFunction Light On Strength Shadows Temperature Light%20Color Target%20Point Pitch Yaw Radius Angle))